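; Melee attack gameplay ability that faces the avatar toward its combat target and plays a random tagged attack montage.
; On the montage's socket-tag gameplay event, it gathers live players within a small radius of that combat socket and damages non-friendly ones.
; A hit fires a MeleeImpact gameplay cue carrying the montage tag, socket location and combat target.
; The ability ends after the hit check or when the montage finishes, blends out or is interrupted.
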(event `self.K2_ActivateAbility`
  (bind _returnvalue (`self.GetAvatarActorFromActorInfo`))
  (bind _returnvalue_2 (`self.GetAvatarActorFromActorInfo`))
  (bind (_taggedmontage_montage _taggedmontage_montagetag) (break `TaggedMontage` (`self.TaggedMontage`)))
  (set `self.bHasTarget` false)
  (bind _returnvalue_3 (message `EnemyInterface.GetCombatTarget` (`self.GetAvatarActorFromActorInfo`)))
  (message `CombatInterface.UpdateFacingTarget` _returnvalue_3 (`Actor.K2_GetActorLocation` _returnvalue_3))
  (bind _returnvalue_4 (message `CombatInterface.GetAttackMontages` (`self.GetAvatarActorFromActorInfo`)))
  (bind _outitem (`KismetArrayLibrary.Array_Random` _returnvalue_4))
  (set `self.TaggedMontage` _outitem)
  (bind (_montage _montagetag _sockettag) (break `TaggedMontage` _outitem))
  (`AbilityTask_PlayMontageAndWait.CreatePlayMontageAndWaitProxy` "None" _montage
    (:`then`
      (`AbilityTask_WaitGameplayEvent.WaitGameplayEvent` _sockettag null
        (:`EventReceived`
          (bind _returnvalue_5 (message `CombatInterface.GetCombatSocketLocation` _returnvalue_2 _sockettag))
          (set `self.Socket Location` _returnvalue_5)
          (bind _outoverlappingactors (`AuraAbilitySystemBlueprintLibrary.GetLivePlayersWithinRadius` _returnvalue_2 (`|MakeArray` _returnvalue_2) 60.0 _returnvalue_5))
          (for _array_element _outoverlappingactors
            (if (`AuraAbilitySystemBlueprintLibrary.IsNotFriend` (`self.GetAvatarActorFromActorInfo`) _array_element)
              (`self.CauseDamage` _array_element)
              (set `self.bHasTarget` true)))
          (if (`self.bHasTarget`)
            (bind _returnvalue_6 (message `EnemyInterface.GetCombatTarget` _returnvalue))
            (`self.K2_ExecuteGameplayCueWithParams` (struct :`TagName` "GameplayCue.MeleeImpact") (`AbilitySystemBlueprintLibrary.MakeGameplayCueParameters` 0.0 0.0 (struct) (struct) (struct) (`BlueprintGameplayTagLibrary.MakeGameplayTagContainerFromTag` _taggedmontage_montagetag) (struct) (`self.Socket Location`) (0.0 0.0 0.0) null _returnvalue _returnvalue_6)))
          (`self.K2_EndAbility`))))
    (:`OnCompleted`
      (`self.K2_EndAbility` :!label _label))
    (:`OnBlendOut`
      (goto _label))
    (:`OnInterrupted`
      (goto _label))
    (:`OnCancelled`
      (goto _label))))