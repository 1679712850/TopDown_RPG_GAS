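; GA_RangedAttack is a gameplay ability for a ranged attack, currently ending in a debug sphere rather than a projectile or damage.
; On activation it turns the avatar toward its combat target through interface messages, then plays a random attack montage.
; It waits for a montage-tag gameplay event and draws the sphere at that tag's combat socket.
; Montage and tag come from separate Random evaluations, so they may not match.
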(event `self.K2_ActivateAbility`
  (bind _returnvalue (message `EnemyInterface.GetCombatTarget` (`self.GetAvatarActorFromActorInfo`)))
  (message `CombatInterface.UpdateFacingTarget` _returnvalue (`Actor.K2_GetActorLocation` _returnvalue))
  (bind _returnvalue_2 (message `CombatInterface.GetAttackMontages` (`self.GetAvatarActorFromActorInfo`)))
  (bind (_montage _montagetag) (break `TaggedMontage` (`KismetArrayLibrary.Array_Random` _returnvalue_2)))
  (`AbilityTask_PlayMontageAndWait.CreatePlayMontageAndWaitProxy` "None" _montage
    (:`then`
      (`AbilityTask_WaitGameplayEvent.WaitGameplayEvent` _montagetag null
        (:`EventReceived`
          (bind _returnvalue_3 (message `CombatInterface.GetCombatSocketLocation` (`self.GetAvatarActorFromActorInfo`) _montagetag))
          (`KismetSystemLibrary.DrawDebugSphere` _returnvalue_3 30.0 12 (struct :`R` 1.0 :`G` 1.0 :`B` 1.0 :`A` 1.0) 3.0))))))