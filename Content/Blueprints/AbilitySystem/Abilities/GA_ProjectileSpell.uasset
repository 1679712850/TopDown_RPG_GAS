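; Gameplay ability that casts a Fire Bolt projectile spell toward the point under the mouse.
; On activation, a target data task supplies the hit location, and the avatar updates its facing target through CombatInterface.
; It plays the cast montage with the generic PlayMontage node, then waits for the montage's gameplay event.
; That event spawns the projectile from the weapon socket toward the location and ends the ability.
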(event `self.K2_ActivateAbility`
  (bind (_asynctaskproxy _data) (`TargetDataUnderMouse.CreateTargetDataUnderMouse`)
    (:`then`
      (set `self.TargetLocation` (`.Location` (`GameplayStatics.BreakHitResult` (`AbilitySystemBlueprintLibrary.GetHitResultFromTargetData` _data))))
      (bind _ascombat_interface (cast `CombatInterface` (`self.GetAvatarActorFromActorInfo`)))
      (`CombatInterface.UpdateFacingTarget` _ascombat_interface (`self.TargetLocation`))
      (`|PlayMontage` (`Character.Mesh` (cast `Character` (`self.GetAvatarActorFromActorInfo`) :!pure true)) "/Game/Assets/Characters/Aura/Animations/Abilities/AM_Cast_FireBolt.AM_Cast_FireBolt"
        (:`then`
          (`AbilityTask_WaitGameplayEvent.WaitGameplayEvent` (struct :`TagName` "Event.Montage.FireBolt") null
            (:`EventReceived`
              (`self.SpawnProjectile` (`self.TargetLocation`) (`BlueprintGameplayTagLibrary.MakeLiteralGameplayTag` (struct :`TagName` "CombatSocket.Weapon")))
              (`self.K2_EndAbility`))))))))