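; Gameplay ability in which a shaman summons random minions with AI controllers around spawn points.
; It shuffles the locations, shows a ground Niagara effect at each, and plays the summon montage.
; The montage's gameplay event starts a delayed loop that spawns minions one by one, facing away from the summoner.
; Each spawn increments the summoner's minion count, and each minion's destruction decrements it.
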(event `self.K2_ActivateAbility`
  (bind _returnvalue (+ (`|GetArrayItem` (`self.Spawn Locations`) (`self.Spawn Location Index`)) (0.0 0.0 70.0)))
  (bind _returnvalue_2 (`self.GetSpawnLocations`))
  (bind _output_get (set `self.Spawn Locations` _returnvalue_2))
  (`KismetArrayLibrary.Array_Shuffle` _output_get)
  (for _array_element (`self.Spawn Locations`)
    (`NiagaraFunctionLibrary.SpawnSystemAtLocation` "/Game/Assets/Effects/Combat/NS_GroundSummon.NS_GroundSummon" _array_element))
  (`AbilityTask_PlayMontageAndWait.CreatePlayMontageAndWaitProxy` "None" "/Game/Assets/Enemies/Shaman/Animations/AM_Shaman_Summon.AM_Shaman_Summon"
    (:`then`
      (`AbilityTask_WaitGameplayEvent.WaitGameplayEvent` (struct :`TagName` "Montage.Attack.1") null
        (:`EventReceived`
          (if (< (`self.Spawn Location Index`) (`KismetArrayLibrary.Array_Length` (`self.Spawn Locations`))) :!label _label
            (bind _returnvalue_3 (`|SpawnActorFromClass` (`self.GetRandomMinionClass`) (`KismetMathLibrary.MakeTransform` _returnvalue (`KismetMathLibrary.FindLookAtRotation` (`Actor.K2_GetActorLocation` (`self.GetAvatarActorFromActorInfo`)) _returnvalue)) "AlwaysSpawn" "MultiplyWithRoot" null null))
            (add `Actor.OnDestroyed` _returnvalue_3 (delegate `OnDestroyed_Event`))
            (`Pawn.SpawnDefaultController` _returnvalue_3)
            (message `CombatInterface.IncremenetMinionCount` (`self.GetAvatarActorFromActorInfo`) 1)
            (`/Engine/EditorBlueprintResources/StandardMacros.IncrementInt` (`self.Spawn Location Index`)
              (:`  `
                (`KismetSystemLibrary.Delay` 0.2)
                (goto _label)))))))))

(event `OnDestroyed_Event`
  (params (DestroyedActor :type "Actor Object Reference"))
  (message `CombatInterface.IncremenetMinionCount` (`self.GetAvatarActorFromActorInfo`) -1))