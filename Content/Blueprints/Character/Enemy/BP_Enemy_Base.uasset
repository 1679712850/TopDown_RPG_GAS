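; Base enemy Blueprint that handles spawn scale-in, motion-warp facing, body and weapon dissolves, and loot drops.
; Timelines scale the mesh on BeginPlay and drive the Dissolve parameter on dynamic materials.
; A custom event gets items from the loot tiers, then a looping timer spawns them one by one, evenly fanned around the enemy at random distances.
; Spawned AuraEffectActors take the enemy's level; the LootLevelOverride branch is empty.
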(event `CustomEvent`
  (bind _returnvalue (`AuraAbilitySystemBlueprintLibrary.GetLootTiers` null))
  (`/Engine/EditorBlueprintResources/StandardMacros.IsValid` _returnvalue
    (:`Is Valid`
      (bind _returnvalue_2 (`LootTiers.GetLootItems` _returnvalue))
      (set `self.NewVar` _returnvalue_2)
      (set `self.LootRotations` (`self.GetLootRotations` _))
      (set `self.SpawnLoopCount` 0)
      (bind _returnvalue_3 (`KismetSystemLibrary.K2_SetTimerDelegate` (delegate `SpawnLootItem`) 0.1 true))
      (set `self.LootTimer` _returnvalue_3)
      (`self.SpawnLootItem`))))

(event `SpawnLootItem`
  (bind (_lootclass _blootleveloverride) (break `LootItem` (`|GetArrayItem` (`self.NewVar`) (`self.SpawnLoopCount`))))
  (if (< (`self.SpawnLoopCount`) (`KismetArrayLibrary.Array_Length` (`self.NewVar`)))
    (bind _returnvalue (`|SpawnActorFromClass` _lootclass (`self.GetLootTransform` (`self.SpawnLoopCount`)) "AlwaysSpawn" "MultiplyWithRoot" null null))
    (bind _asaura_effect_actor (cast `AuraEffectActor` _returnvalue)
      (:`then`
        (set `AuraEffectActor.EffectLevel` (`KismetMathLibrary.Conv_IntToDouble` (`self.Level`)) _asaura_effect_actor)
        (if _blootleveloverride
          _
          (else
            _)))
      (:`CastFailed`
        _))
    (`/Engine/EditorBlueprintResources/StandardMacros.IncrementInt` (`self.SpawnLoopCount`))
    (else
      (`KismetSystemLibrary.K2_ClearAndInvalidateTimerHandle` (`self.LootTimer`)))))

(event `self.ReceiveBeginPlay`
  (bind (_direction _newtrack_0) (`Timeline|Timeline_1`)
    (:`Update`
      (`SceneComponent.SetRelativeScale3D` (`self.Mesh`) (`KismetMathLibrary.MakeVector` _newtrack_0 _newtrack_0 _newtrack_0)))))

(event `CombatInterface.UpdateFacingTarget`
  (params (Target :type "Vector Structure (by ref)"))
  (`MotionWarpingComponent.AddOrUpdateWarpTargetFromLocation` (`self.MotionWarping`) "FacingTarget" Target))

(event `self.StartDissolveTimeline`
  (params (DynamicMaterialInstance :type "MaterialInstanceDynamic Object Reference"))
  (bind (_direction _newtrack_0) (`Timeline|Timeline`)
    (:`Update`
      (`MaterialInstanceDynamic.SetScalarParameterValue` DynamicMaterialInstance "Dissolve" _newtrack_0))))

(event `self.StartWeaponDissolveTimeline`
  (params (DynamicMaterialInstance :type "MaterialInstanceDynamic Object Reference"))
  (bind (_direction _newtrack_0) (`Timeline|Timeline_0`)
    (:`Update`
      (`MaterialInstanceDynamic.SetScalarParameterValue` DynamicMaterialInstance "Dissolve" _newtrack_0))))

(fn `GetLootRotations`
  (params (TargetArray :type "Array of LootItem Structure (by ref)"))
  (returns (ReturnValue :type "Array of Rotator Structure"))
  (return (`AuraAbilitySystemBlueprintLibrary.EvenlySpacedRotators` (`self.GetActorForwardVector`) (`KismetMathLibrary.Vector_Up`) 360.0 (`KismetArrayLibrary.Array_Length` TargetArray))))

(fn `GetLootTransform`
  (params (LoopCount :type Integer))
  (returns (SpawnTransform :type "Transform Structure"))
  (bind _output (`|GetArrayItem` (`self.LootRotations`) LoopCount))
  (return (`KismetMathLibrary.MakeTransform` (+ (* (`KismetMathLibrary.GetForwardVector` _output) (`KismetMathLibrary.RandomFloatInRange` (`self.Min Spawn Distance`) (`self.Max Spawn Distance`))) (`self.K2_GetActorLocation`)) _output)))

(fn `UserConstructionScript`)