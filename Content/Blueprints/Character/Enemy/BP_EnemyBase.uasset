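; BP_EnemyBase is a base enemy character Blueprint that handles visual effects and attack facing.
; On BeginPlay a timeline animates the mesh's uniform scale.
; UpdateFacingTarget feeds a location into Motion Warping as the "FacingTarget" warp target.
; Separate dissolve events for body and weapon run timelines that drive a "Dissolve" scalar on the supplied dynamic material instance.
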(event `self.ReceiveBeginPlay`
  (bind (_direction _newtrack_0) (`Timeline|Timeline_0`)
    (:`Update`
      (`SceneComponent.SetRelativeScale3D` (`self.Mesh`) (`KismetMathLibrary.MakeVector` _newtrack_0 _newtrack_0 _newtrack_0)))))

(event `CombatInterface.UpdateFacingTarget`
  (params (Target :type "Vector Structure (by ref)"))
  (`MotionWarpingComponent.AddOrUpdateWarpTargetFromLocation` (`self.MotionWarping`) "FacingTarget" Target))

(event `self.StartDissolveTimeline`
  (params (DynamicMaterialInstance :type "MaterialInstanceDynamic Object Reference"))
  (bind (_direction _newtrack_0) (`Timeline|Dissolve Timeline`)
    (:`Update`
      (`MaterialInstanceDynamic.SetScalarParameterValue` DynamicMaterialInstance "Dissolve" _newtrack_0))))

(event `self.StartWeaponDissolveTimeline`
  (params (DynamicMaterialInstance :type "MaterialInstanceDynamic Object Reference"))
  (bind (_direction _newtrack_0) (`Timeline|Timeline`)
    (:`Update`
      (`MaterialInstanceDynamic.SetScalarParameterValue` DynamicMaterialInstance "Dissolve" _newtrack_0))))

(fn `UserConstructionScript`)